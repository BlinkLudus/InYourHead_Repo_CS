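; BP_ShelfFalling is a one-shot scare or set-piece prop whose Locker tips when the Box trigger is overlapped.
; The construction script caches the Locker's relative location, from which MoveComponentTo eases a short shift and tilt for BP_FirstPersonCharacter.
; DoOnce precedes the class check, so any first overlapping actor consumes the trigger.
; A metal impact sound plays at that cached relative location, passed as a world position.
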(event OnComponentBeginOverlap(Box)
  (params (OverlappedComponent :type Primitive%20Component%20Object%20Reference) (OtherActor :type Actor%20Object%20Reference) (OtherComp :type Primitive%20Component%20Object%20Reference) (OtherBodyIndex :type Integer) (bFromSweep :type Boolean) (SweepResult :type Hit%20Result%20Structure%20%28by%20ref%29))
  (Utilities|FlowControl|DoOnce false
    (:Completed
      (if (== (Utilities|GetClass OtherActor) "/Game/ThirdPerson/Blueprints/BP_FirstPersonCharacter.BP_FirstPersonCharacter_C")
        (Components|MoveComponentTo (Variables|Default|GetLocker) (+ (Variables|Default|Getorignal%20location) "10.000000,0.000000,0.000000") "-45.000000,0.000000,0.000000" false true 0.5 false)
        (Audio|PlaySoundatLocation "/Game/Sounds/423117__ogsoundfx__guns-explosions-album-metal-impact-5.423117__ogsoundfx__guns-explosions-album-metal-impact-5" (Variables|Default|Getorignal%20location) "0, 0, 0" 1.0 1.0 0.0 0 0 0 0)))))

(event EventBeginPlay)

(event Collision|EventActorBeginOverlap
  (params (OtherActor :type Actor%20Object%20Reference)))

(event EventTick
  (params (DeltaSeconds :type Float%20%28single-precision%29)))

(fn ConstructionScript
  (Variables|Default|Setorignal%20location (Variables|/Script/Engine.SceneComponent|GetRelativeLocation (Variables|Default|GetLocker))))