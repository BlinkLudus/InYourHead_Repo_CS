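; BP_Door is a sliding door that the first-person character toggles with the Interact input while standing in its Box trigger.
; Overlapping the Box shows front and back text labels and, for that character, enables input on the actor; leaving reverses both.
; Opening or closing slides the door between its construction-time location and a sideways offset, swapping text color and door material between green and red.
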(event OnComponentBeginOverlap(Box)
  (params (OverlappedComponent :type Primitive%20Component%20Object%20Reference) (OtherActor :type Actor%20Object%20Reference) (OtherComp :type Primitive%20Component%20Object%20Reference) (OtherBodyIndex :type Integer) (bFromSweep :type Boolean) (SweepResult :type Hit%20Result%20Structure%20%28by%20ref%29))
  (Rendering|SetVisibility (Variables|Default|GetTextFront) true false)
  (if (== (Utilities|GetClass OtherActor) "/Game/ThirdPerson/Blueprints/BP_FirstPersonCharacter.BP_FirstPersonCharacter_C")
    (Input|EnableInput (Game|GetPlayerController 0))))

(event OnComponentEndOverlap(Box)
  (params (OverlappedComponent :type Primitive%20Component%20Object%20Reference) (OtherActor :type Actor%20Object%20Reference) (OtherComp :type Primitive%20Component%20Object%20Reference) (OtherBodyIndex :type Integer))
  (Rendering|SetVisibility (Variables|Default|GetTextFront) false false)
  (if (== (Utilities|GetClass OtherActor) "/Game/ThirdPerson/Blueprints/BP_FirstPersonCharacter.BP_FirstPersonCharacter_C")
    (Input|DisableInput (Game|GetPlayerController 0))))

(event Custom|Open%20Door
  (Rendering|Components|TextRender|SetTextRenderColor (Variables|Default|GetTextFront) (Math|Color|MakeColor 0 100 0))
  (Rendering|Material|SetMaterial (Variables|Default|GetDoor) 5 "/Game/Materials/M_GreenDoor.M_GreenDoor")
  (Components|MoveComponentTo (Variables|Default|GetDoor) (+ (Variables|Default|GetOriginalLocation) "0.000000,-150.000000,0.000000") "0, 0, 0" false false 1.0 false)
  (Variables|Default|SetIsDoorOpen true))

(event Custom|Close%20Door
  (Rendering|Components|TextRender|SetTextRenderColor (Variables|Default|GetTextFront) (Math|Color|MakeColor 0 0 255))
  (Rendering|Material|SetMaterial (Variables|Default|GetDoor) 5 "/Game/Materials/M_RedDoor.M_RedDoor")
  (Components|MoveComponentTo (Variables|Default|GetDoor) (Variables|Default|GetOriginalLocation) "0, 0, 0" false false 1.0 false)
  (Variables|Default|SetIsDoorOpen false))

(event Input|EnhancedActionEvents|EnhancedInputActionIA_Interact
  (params (ActionValue :type Boolean) (ElapsedSeconds :type Float%20%28double-precision%29) (TriggeredSeconds :type Float%20%28double-precision%29) (InputAction :type Input%20Action%20Object%20Reference :default "/Game/ThirdPerson/Input/Actions/IA_Interact.IA_Interact"))
  (if (Variables|Default|GetIsDoorOpen)
    (CallFunction|CloseDoor)
    (else
      (CallFunction|OpenDoor))))

(fn ConstructionScript
  (Variables|Default|SetOriginalLocation (Variables|/Script/Engine.SceneComponent|GetRelativeLocation (Variables|Default|GetDoor))))