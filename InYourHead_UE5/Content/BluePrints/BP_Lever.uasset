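; BP_Lever is an interactable lever that opens a referenced hatch when the first-person character uses it.
; A sensor overlap toggles a text prompt for any actor and enables or disables the lever's input for the player character.
; The interact action runs once, playing the lever level sequence, hiding the prompt and calling OpenDoor on the hatch.
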(event OnComponentBeginOverlap(LeverSensor)
  (params (OverlappedComponent :type Primitive%20Component%20Object%20Reference) (OtherActor :type Actor%20Object%20Reference) (OtherComp :type Primitive%20Component%20Object%20Reference) (OtherBodyIndex :type Integer) (bFromSweep :type Boolean) (SweepResult :type Hit%20Result%20Structure%20%28by%20ref%29))
  (Rendering|SetVisibility (Variables|Default|GetTextRender) true false)
  (if (== (Utilities|GetClass OtherActor) "/Game/ThirdPerson/Blueprints/BP_FirstPersonCharacter.BP_FirstPersonCharacter_C")
    (Input|EnableInput (Game|GetPlayerController 0))))

(event OnComponentEndOverlap(LeverSensor)
  (params (OverlappedComponent :type Primitive%20Component%20Object%20Reference) (OtherActor :type Actor%20Object%20Reference) (OtherComp :type Primitive%20Component%20Object%20Reference) (OtherBodyIndex :type Integer))
  (Rendering|SetVisibility (Variables|Default|GetTextRender) false false)
  (if (== (Utilities|GetClass OtherActor) "/Game/ThirdPerson/Blueprints/BP_FirstPersonCharacter.BP_FirstPersonCharacter_C")
    (Input|DisableInput (Game|GetPlayerController 0))))

(event Input|EnhancedActionEvents|EnhancedInputActionIA_Interact
  (params (ActionValue :type Boolean) (ElapsedSeconds :type Float%20%28double-precision%29) (TriggeredSeconds :type Float%20%28double-precision%29) (InputAction :type Input%20Action%20Object%20Reference :default "/Game/ThirdPerson/Input/Actions/IA_Interact.IA_Interact"))
  (Utilities|FlowControl|DoOnce false
    (:Completed
      (bind _outactor (Sequencer|Player|CreateLevelSequencePlayer "/Game/LS_Lever.LS_Lever"))
      (Sequencer|Player|Play (Variables|/Script/LevelSequence.LevelSequenceActor|GetSequencePlayer _outactor) :!class /Script/MovieScene.MovieSceneSequencePlayer)
      (Rendering|SetVisibility (Variables|Default|GetTextRender) false false)
      (Default|OpenDoor (Variables|Default|GetHatchRef)))))

(fn ConstructionScript
  (Variables|Default|SetOriginalLocation (Variables|/Script/Engine.SceneComponent|GetRelativeLocation (Variables|Default|GetLever))))