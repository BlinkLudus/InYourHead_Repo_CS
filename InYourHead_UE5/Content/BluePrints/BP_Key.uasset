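; Collectible key card pickup with a low, mid or high security type.
; The construction script tints a dynamic material instance of M_KeyEditable with the colour matching KeyType.
; When BP_FirstPersonCharacter overlaps the sphere, it adds the type to the player's CollectedKeyCards array and destroys itself.
; Before destruction it prints the type and total count, derived from the Add index plus one, in the key's colour.
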(event OnComponentBeginOverlap(Sphere)
  (params (OverlappedComponent :type Primitive%20Component%20Object%20Reference) (OtherActor :type Actor%20Object%20Reference) (OtherComp :type Primitive%20Component%20Object%20Reference) (OtherBodyIndex :type Integer) (bFromSweep :type Boolean) (SweepResult :type Hit%20Result%20Structure%20%28by%20ref%29))
  (bind _asbp_first_person_character (Utilities|Casting|CastToBP_FirstPersonCharacter OtherActor))
  (bind _returnvalue (Utilities|Array|Add (Variables|/Game/ThirdPerson/Blueprints/BP_FirstPersonCharacter.BP_FirstPersonCharacter_C|GetCollectedKeyCards _asbp_first_person_character) (Variables|Default|GetKeyType)))
  (bind _result (Math|Integer|IncrementInt _returnvalue)
    (:%20%20
      (CallFunction|UpdateUI _result)
      (Actor|DestroyActor))))

(event Custom|Update%20UI
  (params (Key%20Count :type Integer))
  (Development|PrintString (Utilities|String|Append (Utilities|String|MakeLiteralString "Collected Key Cards ") (Utilities|String|EnumtoString (Variables|Default|GetKeyType)) (Utilities|String|MakeLiteralString "Total key cards ") (Utilities|String|ToString(Integer) Key%20Count)) true true (Variables|Default|GetKeyColour) 5.0))

(fn ConstructionScript
  (bind _s_keytypecolours (Utilities|Struct|MakeS_KeyTypeColours "(R=0.000000,G=0.087873,B=1.000000,A=1.000000)" "(R=0.901042,G=0.413770,B=0.000000,A=1.000000)" "(R=0.453125,G=0.009832,B=0.000000,A=1.000000)"))
  (bind (_lowsecurity _midsecurity _highsecurity) (Utilities|Struct|BreakS_KeyTypeColours _s_keytypecolours))
  (bind _returnvalue (Rendering|Material|CreateDynamicMaterialInstance (Variables|Default|GetStaticMesh) 0 "/Game/Materials/M_KeyEditable.M_KeyEditable" "None" :!class /Script/Engine.PrimitiveComponent))
  (switch Utilities|FlowControl|Switch|SwitchonE_KeyType (Variables|Default|GetKeyType)
    (:NewEnumerator0
      (Variables|Default|SetKeyColour _lowsecurity))
    (:NewEnumerator1
      (Variables|Default|SetKeyColour _midsecurity))
    (:NewEnumerator2
      (Variables|Default|SetKeyColour _highsecurity)))
  (Rendering|Material|SetVectorParameterValue _returnvalue "Base Color" (Variables|Default|GetKeyColour) :!class /Script/Engine.MaterialInstanceDynamic))