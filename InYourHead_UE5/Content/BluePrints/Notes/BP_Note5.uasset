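; BP_Note5 is a readable note that the player opens through an interact input while standing in its Box trigger.
; Overlap toggles the Interact prompt for any actor and enables input only for BP_FirstPersonCharacter.
; Reading passes a DoOnce and an IsNoteOpen check, then shows WBP_Note4 (not a Note5 widget) and blocks look and move input.
; The close input removes the widget, restores control and resets the DoOnce.
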(event OnComponentBeginOverlap(Box)
  (params (OverlappedComponent :type Primitive%20Component%20Object%20Reference) (OtherActor :type Actor%20Object%20Reference) (OtherComp :type Primitive%20Component%20Object%20Reference) (OtherBodyIndex :type Integer) (bFromSweep :type Boolean) (SweepResult :type Hit%20Result%20Structure%20%28by%20ref%29))
  (Rendering|SetVisibility (Variables|Default|GetInteract) true false)
  (if (== (Utilities|GetClass OtherActor) "/Game/ThirdPerson/Blueprints/BP_FirstPersonCharacter.BP_FirstPersonCharacter_C")
    (Input|EnableInput (Game|GetPlayerController 0))))

(event OnComponentEndOverlap(Box)
  (params (OverlappedComponent :type Primitive%20Component%20Object%20Reference) (OtherActor :type Actor%20Object%20Reference) (OtherComp :type Primitive%20Component%20Object%20Reference) (OtherBodyIndex :type Integer))
  (Rendering|SetVisibility (Variables|Default|GetInteract) false false)
  (if (== (Utilities|GetClass OtherActor) "/Game/ThirdPerson/Blueprints/BP_FirstPersonCharacter.BP_FirstPersonCharacter_C")
    (Input|DisableInput (Game|GetPlayerController 0))))

(event Custom|ReadNote
  (bind _returnvalue (Game|GetPlayerController 0))
  (Utilities|FlowControl|DoOnce false
    (:Completed
      (if (not (Variables|Default|GetIsNoteOpen?))
        (bind _returnvalue_2 (UserInterface|CreateWidget "/Game/BluePrints/Notes/WBP_Note4.WBP_Note4_C" (Game|GetPlayerController 0)))
        (UserInterface|Viewport|AddtoViewport _returnvalue_2 0)
        (Input|SetIgnoreLookInput _returnvalue true)
        (Input|SetIgnoreMoveInput _returnvalue true)))))

(event Input|EnhancedActionEvents|EnhancedInputActionIA_Interact
  (params (ActionValue :type Boolean) (ElapsedSeconds :type Float%20%28double-precision%29) (TriggeredSeconds :type Float%20%28double-precision%29) (InputAction :type Input%20Action%20Object%20Reference :default "/Game/ThirdPerson/Input/Actions/IA_Interact.IA_Interact"))
  (CallFunction|ReadNote))

(event Input|EnhancedActionEvents|EnhancedInputActionIA_CloseNote
  (params (ActionValue :type Boolean) (ElapsedSeconds :type Float%20%28double-precision%29) (TriggeredSeconds :type Float%20%28double-precision%29) (InputAction :type Input%20Action%20Object%20Reference :default "/Game/ThirdPerson/Input/Actions/IA_CloseNote.IA_CloseNote"))
  (bind _returnvalue (Game|GetPlayerController 0))
  (bind _returnvalue_2 (Game|GetPlayerController 0))
  (Widget|RemovefromParent (stale Custom|ReadNote _returnvalue_2))
  (Input|SetIgnoreLookInput _returnvalue_2 false)
  (Input|SetIgnoreMoveInput _returnvalue_2 false)
  (Utilities|FlowControl|DoOnce false) ; enters at Reset
)

(event EventBeginPlay)

(fn ConstructionScript)