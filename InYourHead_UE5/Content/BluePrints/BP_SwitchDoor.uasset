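; BP_SwitchDoor is a sliding door that opens and closes through its OpenDoor and CloseDoor events, with sound feedback.
; The construction script caches the door mesh's starting relative location as the closed position.
; Each event plays the sound, swaps one material slot to green or red, and uses MoveComponentTo to slide the door sideways or back.
; An IsDoorOpen flag records the current state.
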(event Custom|Open%20Door
  (Audio|Components|Audio|Play (Variables|Default|GetSound) 0.0)
  (Rendering|Material|SetMaterial (Variables|Default|GetDoor) 5 "/Game/Materials/M_GreenDoor.M_GreenDoor")
  (Components|MoveComponentTo (Variables|Default|GetDoor) (+ (Variables|Default|GetOriginalLocation) "0.000000,-150.000000,0.000000") "0, 0, 0" false false 1.0 false)
  (Variables|Default|SetIsDoorOpen true))

(event Custom|Close%20Door
  (Audio|Components|Audio|Play (Variables|Default|GetSound) 0.0)
  (Rendering|Material|SetMaterial (Variables|Default|GetDoor) 5 "/Game/Materials/M_RedDoor.M_RedDoor")
  (Components|MoveComponentTo (Variables|Default|GetDoor) (Variables|Default|GetOriginalLocation) "0, 0, 0" false false 1.0 false)
  (Variables|Default|SetIsDoorOpen false))

(fn ConstructionScript
  (Variables|Default|SetOriginalLocation (Variables|/Script/Engine.SceneComponent|GetRelativeLocation (Variables|Default|GetDoor))))