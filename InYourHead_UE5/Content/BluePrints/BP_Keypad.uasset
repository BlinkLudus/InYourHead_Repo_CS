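; Interactable keypad that lets the first-person character open a key code panel when nearby.
; Box overlap shows or hides a text component for any actor, but toggles input only for the character.
; IA_Interact flip-flops between creating the WBP_KeyCodePanel with cursor and Game-and-UI input, and removing it.
; Leaving the box also closes the panel and restores game-only input, without resetting the FlipFlop.
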(event OnComponentBeginOverlap(Box)
  (params (OverlappedComponent :type Primitive%20Component%20Object%20Reference) (OtherActor :type Actor%20Object%20Reference) (OtherComp :type Primitive%20Component%20Object%20Reference) (OtherBodyIndex :type Integer) (bFromSweep :type Boolean) (SweepResult :type Hit%20Result%20Structure%20%28by%20ref%29))
  (Rendering|SetVisibility (Variables|Default|GetText) true false)
  (if (== (Utilities|GetClass OtherActor) "/Game/ThirdPerson/Blueprints/BP_FirstPersonCharacter.BP_FirstPersonCharacter_C")
    (Input|EnableInput (Game|GetPlayerController 0))))

(event OnComponentEndOverlap(Box)
  (params (OverlappedComponent :type Primitive%20Component%20Object%20Reference) (OtherActor :type Actor%20Object%20Reference) (OtherComp :type Primitive%20Component%20Object%20Reference) (OtherBodyIndex :type Integer))
  (bind _returnvalue (Game|GetPlayerController 0))
  (Rendering|SetVisibility (Variables|Default|GetText) false false)
  (if (== (Utilities|GetClass OtherActor) "/Game/ThirdPerson/Blueprints/BP_FirstPersonCharacter.BP_FirstPersonCharacter_C")
    (Input|DisableInput (Game|GetPlayerController 0))
    (Widget|RemovefromParent (stale Input|EnhancedActionEvents|EnhancedInputActionIA_Interact _returnvalue_2))
    (Input|SetInputModeGameOnly _returnvalue false)
    (Variables|/Script/Engine.PlayerController|SetbShowMouseCursor _returnvalue false)))

(event Input|EnhancedActionEvents|EnhancedInputActionIA_Interact
  (params (ActionValue :type Boolean) (ElapsedSeconds :type Float%20%28double-precision%29) (TriggeredSeconds :type Float%20%28double-precision%29) (InputAction :type Input%20Action%20Object%20Reference :default "/Game/ThirdPerson/Input/Actions/IA_Interact.IA_Interact"))
  (bind _returnvalue (Game|GetPlayerController 0))
  (:Started
    (Utilities|FlowControl|FlipFlop
      (:A
        (bind _returnvalue_2 (UserInterface|CreateWidget "/Game/BluePrints/UI/WBP_KeyCodePanel.WBP_KeyCodePanel_C"))
        (UserInterface|Viewport|AddtoViewport _returnvalue_2 0)
        (Input|SetInputModeGameandUI _returnvalue _returnvalue_2 "DoNotLock" true false)
        (Variables|/Script/Engine.PlayerController|SetbShowMouseCursor _returnvalue true))
      (:B
        (Widget|RemovefromParent _returnvalue_2)
        (Input|SetInputModeGameOnly _returnvalue false)
        (Variables|/Script/Engine.PlayerController|SetbShowMouseCursor _returnvalue false)))))

(fn ConstructionScript)