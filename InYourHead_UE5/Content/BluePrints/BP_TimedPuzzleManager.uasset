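; Timed switch puzzle manager that opens a door once enough switches are activated before a countdown expires.
; The first activation passes a DoOnce to create the timer widget and start the countdown, which Tick decrements through a one-second Delay.
; Reaching the switch total opens the door, removes the widget and destroys the manager.
; At zero, it resets every switch, hides the widget and re-arms the DoOnce.
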(event Custom|Start%20Puzzle%20Timer
  ;[1 1 1] Start puzzle timer when player activates switch
  (Utilities|FlowControl|DoOnce false
    (:Completed
      (bind _returnvalue (UserInterface|CreateWidget "/Game/BluePrints/WBP_Timer.WBP_Timer_C" (Game|GetPlayerController 0)))
      (bind _output_get (Variables|Default|SetHUDref _returnvalue))
      (UserInterface|Viewport|AddtoViewport _output_get 0)
      (bind _output_get_2 (Variables|Default|SetCurrentTime (Variables|Default|GetMaxTime)))
      (bind _returnvalue_2 (Utilities|Time|SetTimerbyEvent 0 _output_get_2))
      (Variables|Default|SetNewVar _returnvalue_2)
      (Variables|Default|SetbTimerActive true))))

(event Custom|Reset%20Switches
  ;[1 1 1] Reset switches if time runs out
  (for _array_element (Variables|Default|GetSwitches)
    (Variables|Default|SetActivatedSwitches 0)
    (Default|Reset _array_element)
    (CallFunction|ResetTimer)
    ;[1 1 1] Start puzzle timer when player activates switch
    (Utilities|FlowControl|DoOnce false) ; enters at Reset
  ))

(event Custom|Switch%20Activated
  (bind _hudref (Variables|Default|GetHudRef))
  ;[1 1 1] Player activates switches -> starts puzzle timer
  (CallFunction|StartPuzzleTimer)
  (Variables|Default|SetActivatedSwitches (+ (Variables|Default|GetActivatedSwitches) 1))
  (if (== (Variables|Default|GetActivatedSwitches) (Variables|Default|GetMaxSwitches))
    (Variables|Default|SetPuzzleComplete true)
    (Default|OpenDoor (Variables|Default|GetDoorRef))
    (Widget|SetVisibility _hudref "Hidden")
    (Widget|RemovefromParent _hudref)
    (Actor|DestroyActor)))

(event Custom|Reset%20Timer
  (bind _hudref (Variables|Default|GetHudRef))
  ;[1 1 1] Reset the timer when it runs out
  (Variables|Default|SetbTimerActive false)
  (Variables|Default|SetMaxTime (Variables|Default|GetMaxTime))
  (Widget|SetVisibility _hudref "Hidden")
  (Widget|RemovefromParent _hudref))

(event EventBeginPlay
  (Variables|Default|SetSwitches (Variables|Default|GetSwitches)))

(event EventTick
  (params (DeltaSeconds :type Float%20%28single-precision%29))
  ;[1 1 1] Set timer
  (Utilities|FlowControl|Delay 1.0)
  (if (Variables|Default|GetbTimerActive)
    (Variables|Default|SetCurrentTime (- (Variables|Default|GetCurrentTime) 1.0))
    (Rendering|Components|TextRender|SetText (Variables|/Game/BluePrints/WBP_Timer.WBP_Timer_C|GetSecondsText (Variables|Default|GetHudRef)) (Utilities|Text|ToText(Float) (Variables|Default|GetCurrentTime) "HalfToEven"))
    (if (<= (Variables|Default|GetCurrentTime) 0.0)
      (CallFunction|ResetSwitches))))

(fn ConstructionScript)

(fn StartTimer)