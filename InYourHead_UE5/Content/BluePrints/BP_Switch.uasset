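; A one-shot interactable switch that reports its activation to a puzzle manager.
; Entering its box trigger shows a text prompt and, for the first-person character, enables Interact input; leaving reverses both.
; Interacting turns the cube green, notifies the referenced puzzle manager and turns a light mesh on the referenced light actor green.
; Reset restores the switch's red material and activation state but leaves that light unchanged.
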(event OnComponentBeginOverlap(Box)
  (params (OverlappedComponent :type Primitive%20Component%20Object%20Reference) (OtherActor :type Actor%20Object%20Reference) (OtherComp :type Primitive%20Component%20Object%20Reference) (OtherBodyIndex :type Integer) (bFromSweep :type Boolean) (SweepResult :type Hit%20Result%20Structure%20%28by%20ref%29))
  (Rendering|SetVisibility (Variables|Default|GetTextRender) true false)
  (if (== (Utilities|GetClass OtherActor) "/Game/ThirdPerson/Blueprints/BP_FirstPersonCharacter.BP_FirstPersonCharacter_C")
    (Input|EnableInput (Game|GetPlayerController 0))))

(event OnComponentEndOverlap(Box)
  (params (OverlappedComponent :type Primitive%20Component%20Object%20Reference) (OtherActor :type Actor%20Object%20Reference) (OtherComp :type Primitive%20Component%20Object%20Reference) (OtherBodyIndex :type Integer))
  (Rendering|SetVisibility (Variables|Default|GetTextRender) false false)
  (if (== (Utilities|GetClass OtherActor) "/Game/ThirdPerson/Blueprints/BP_FirstPersonCharacter.BP_FirstPersonCharacter_C")
    (Input|DisableInput (Game|GetPlayerController 0))))

(event Custom|Reset
  (Rendering|Material|SetMaterial (Variables|Default|GetCube) 0 "/Game/Materials/M_RedDoor.M_RedDoor")
  (Variables|Default|SetbIsActivated false))

(event Custom|SwitchLightActivated
  (Rendering|Material|SetMaterial (Variables|/Game/BluePrints/BP_SwitchLights.BP_SwitchLights_C|GetLight1 (Variables|Default|GetRefLight)) 0 "/Game/Materials/M_GreenDoor.M_GreenDoor"))

(event Input|EnhancedActionEvents|EnhancedInputActionIA_Interact
  (params (ActionValue :type Boolean) (ElapsedSeconds :type Float%20%28double-precision%29) (TriggeredSeconds :type Float%20%28double-precision%29) (InputAction :type Input%20Action%20Object%20Reference :default "/Game/ThirdPerson/Input/Actions/IA_Interact.IA_Interact"))
  (if (not (Variables|Default|GetbIsActivated))
    (Variables|Default|SetbIsActivated true)
    (Rendering|Material|SetMaterial (Variables|Default|GetCube) 0 "/Game/Materials/M_GreenDoor.M_GreenDoor")
    (Default|SwitchActivated (Variables|Default|GetPuzzleManagerREF))
    (CallFunction|SwitchLightActivated)))

(fn ConstructionScript)