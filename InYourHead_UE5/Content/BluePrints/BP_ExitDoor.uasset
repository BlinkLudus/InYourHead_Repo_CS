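; BP_ExitDoor is an exit door that slides open along its local Y axis with a sound and a green material swap.
; A Box overlap shows front and back text for any actor and enables input on the door while BP_FirstPersonCharacter is inside, though no input events appear here.
; The custom OpenDoor event moves the door relative to the location cached in the construction script, with no closing logic.
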(event OnComponentBeginOverlap(Box)
  (params (OverlappedComponent :type Primitive%20Component%20Object%20Reference) (OtherActor :type Actor%20Object%20Reference) (OtherComp :type Primitive%20Component%20Object%20Reference) (OtherBodyIndex :type Integer) (bFromSweep :type Boolean) (SweepResult :type Hit%20Result%20Structure%20%28by%20ref%29))
  (Rendering|SetVisibility (Variables|Default|GetTextBack) true false)
  (if (== (Utilities|GetClass OtherActor) "/Game/ThirdPerson/Blueprints/BP_FirstPersonCharacter.BP_FirstPersonCharacter_C")
    (Input|EnableInput (Game|GetPlayerController 0))))

(event OnComponentEndOverlap(Box)
  (params (OverlappedComponent :type Primitive%20Component%20Object%20Reference) (OtherActor :type Actor%20Object%20Reference) (OtherComp :type Primitive%20Component%20Object%20Reference) (OtherBodyIndex :type Integer))
  (Rendering|SetVisibility (Variables|Default|GetTextBack) false false)
  (if (== (Utilities|GetClass OtherActor) "/Game/ThirdPerson/Blueprints/BP_FirstPersonCharacter.BP_FirstPersonCharacter_C")
    (Input|DisableInput (Game|GetPlayerController 0))))

(event Custom|Open%20Door
  (Audio|Components|Audio|Play (Variables|Default|GetDoorSound) 0.0)
  (Rendering|Material|SetMaterial (Variables|Default|GetDoor) 5 "/Game/Materials/M_GreenDoor.M_GreenDoor")
  (Components|MoveComponentTo (Variables|Default|GetDoor) (+ (Variables|Default|GetOriginalLocation) "0.000000,-150.000000,0.000000") "0, 0, 0" false false 1.0 false))

(fn ConstructionScript
  (Variables|Default|SetOriginalLocation (Variables|/Script/Engine.SceneComponent|GetRelativeLocation (Variables|Default|GetDoor))))