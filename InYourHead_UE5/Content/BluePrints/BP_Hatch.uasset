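; BP_Hatch is a hatch door that opens and closes through OpenDoor and CloseDoor events.
; Each event recolors TextFront (green to open, red to close), moves the Hatch component with MoveComponentTo and sets IsDoorOpen.
; The construction script caches the hatch's relative location, so opening offsets and rotates from it and closing returns to it.
; Leftover logic for toggling text visibility and player input is unconnected and never runs.
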(event Custom|Open%20Door
  (Rendering|Components|TextRender|SetTextRenderColor (Variables|Default|GetTextFront) (Math|Color|MakeColor 0 100 0))
  (Components|MoveComponentTo (Variables|Default|GetHatch) (+ (Variables|Default|GetOriginalLocation) "-150.000000,0.000000,0.000000") "100.000000,0.000000,0.000000" false false 3.0 false)
  (Variables|Default|SetIsDoorOpen true))

(event Custom|Close%20Door
  (Rendering|Components|TextRender|SetTextRenderColor (Variables|Default|GetTextFront) (Math|Color|MakeColor 0 0 255))
  (Components|MoveComponentTo (Variables|Default|GetHatch) (Variables|Default|GetOriginalLocation) "0, 0, 0" false false 1.0 false)
  (Variables|Default|SetIsDoorOpen false))

(fn ConstructionScript
  (Variables|Default|SetOriginalLocation (Variables|/Script/Engine.SceneComponent|GetRelativeLocation (Variables|Default|GetHatch))))