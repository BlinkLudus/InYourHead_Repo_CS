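; BP_Button is an interactable button that silences an alarm sound.
; Its Box trigger shows a TextRender while overlapped by any actor, and enables player 0's input on the button only while BP_FirstPersonCharacter is inside.
; IA_Interact passes through a DoOnce that is never reset, so it plays a switch sound and stops the alarm cue a single time.
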(event OnComponentBeginOverlap(Box)
  (params (OverlappedComponent :type Primitive%20Component%20Object%20Reference) (OtherActor :type Actor%20Object%20Reference) (OtherComp :type Primitive%20Component%20Object%20Reference) (OtherBodyIndex :type Integer) (bFromSweep :type Boolean) (SweepResult :type Hit%20Result%20Structure%20%28by%20ref%29))
  (Rendering|SetVisibility (Variables|Default|GetTextRender) true false)
  (if (== (Utilities|GetClass OtherActor) "/Game/ThirdPerson/Blueprints/BP_FirstPersonCharacter.BP_FirstPersonCharacter_C")
    (Input|EnableInput (Game|GetPlayerController 0))))

(event OnComponentEndOverlap(Box)
  (params (OverlappedComponent :type Primitive%20Component%20Object%20Reference) (OtherActor :type Actor%20Object%20Reference) (OtherComp :type Primitive%20Component%20Object%20Reference) (OtherBodyIndex :type Integer))
  (Rendering|SetVisibility (Variables|Default|GetTextRender) false false)
  (if (== (Utilities|GetClass OtherActor) "/Game/ThirdPerson/Blueprints/BP_FirstPersonCharacter.BP_FirstPersonCharacter_C")
    (Input|DisableInput (Game|GetPlayerController 0))))

(event Custom|StopAlarm
  (Audio|Components|Audio|Stop (Variables|Default|Get316835__lalks__alarm-01-long_Cue)))

(event Input|EnhancedActionEvents|EnhancedInputActionIA_Interact
  (params (ActionValue :type Boolean) (ElapsedSeconds :type Float%20%28double-precision%29) (TriggeredSeconds :type Float%20%28double-precision%29) (InputAction :type Input%20Action%20Object%20Reference :default "/Game/ThirdPerson/Input/Actions/IA_Interact.IA_Interact"))
  (Utilities|FlowControl|DoOnce false
    (:Completed
      (Audio|PlaySound2D "/Game/Sounds/kijjaz-electrical-cutout-box-switch-on-and-off.kijjaz-electrical-cutout-box-switch-on-and-off" 1.0 1.0 0.0 0 0)
      (CallFunction|StopAlarm))))

(fn ConstructionScript)